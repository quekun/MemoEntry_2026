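; Main menu player controller for TankHero that puts up the opening UI when play begins.
; It reads GoDirectlyToLevelSelect from TankHeroGameInstance to show either the level select or the main menu widget, then switches input to UI only.
; The level select branch sets that flag to true again rather than clearing it.
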(event `self.ReceiveBeginPlay`
  (bind _astank_hero_game_instance (cast `TankHeroGameInstance` (`GameplayStatics.GetGameInstance`)))
  (if (`TankHeroGameInstance.bGoDirectlyToLevelSelect` _astank_hero_game_instance)
    (bind _returnvalue (`|CreateWidget` "/Game/MyStuff/Blueprints/WBP_LevelSelect.WBP_LevelSelect_C"))
    (`UserWidget.AddToViewport` _returnvalue 0)
    (set `TankHeroGameInstance.bGoDirectlyToLevelSelect` true _astank_hero_game_instance)
    (else
      (bind _returnvalue_2 (`|CreateWidget` "/Game/MyStuff/Blueprints/WBP_MainMenu.WBP_MainMenu_C"))
      (`UserWidget.AddToViewport` _returnvalue_2 0)))
  (`WidgetBlueprintLibrary.SetInputMode_UIOnlyEx` (`GameplayStatics.GetPlayerController` 0) null))

(fn `UserConstructionScript`)